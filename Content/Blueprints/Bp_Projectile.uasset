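; Projectile actor that delivers a Fire hit effect to environment objects it touches.
; On Sphere overlap, it sends HitEffectMessage with Fire to actors implementing BPI_HitEnvi, then destroys itself; other actors are ignored.
; The construction script assigns configurable Niagara systems to the Niagara and NiagaraHit components, though the graph never explicitly triggers the hit effect.
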(event OnComponentBeginOverlap(Sphere)
  (params (OverlappedComponent :type Primitive%20Component%20Object%20Reference) (OtherActor :type Actor%20Object%20Reference) (OtherComp :type Primitive%20Component%20Object%20Reference) (OtherBodyIndex :type Integer) (bFromSweep :type Boolean) (SweepResult :type Hit%20Result%20Structure%20%28by%20ref%29))
  (if (Utilities|DoesObjectImplementInterface OtherActor "/Game/Blueprints/Envi/BPI_HitEnvi.BPI_HitEnvi_C")
    (Class|BPIHitEnvi|HitEffect(Message) OtherActor (Variables|Default|GetFire?))
    (Actor|DestroyActor)))

(fn ConstructionScript
  (Class|NiagaraComponent|SetAsset (Variables|Default|GetNiagara) (Variables|Default|GetNiagaraSystem) true)
  (Class|NiagaraComponent|SetAsset (Variables|Default|GetNiagaraHit) (Variables|Default|GetNiagaraSystemHit) true))