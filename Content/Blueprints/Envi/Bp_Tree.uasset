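; Tree environment actor that burns away when struck by fire.
; The first HitEffect call with Fire set latches a Hit flag and spawns a constant-fire Niagara system at the tree's location.
; A two-second one-shot timer then calls DestroyTree, which destroys the actor and the spawned effect component.
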(event Custom|DestroyTree
  (Actor|DestroyActor)
  (Components|DestroyComponent (stale EventHitEffect _returnvalue)))

(event EventHitEffect
  (params (Fire? :type Boolean))
  (if (and Fire? (not (Variables|Default|GetHit)))
    (Variables|Default|SetHit true)
    (bind _returnvalue (Niagara|SpawnSystematLocation "/Game/EnergyBeam/NS/NS_Hit_Constant_Fire.NS_Hit_Constant_Fire" (Transformation|GetActorLocation)))
    (Utilities|Time|SetTimerbyEvent (delegate Custom|DestroyTree) 2.0)))

(fn ConstructionScript
  (|CallParentFunction))